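; PartyGoer is a pawn that chases the player once its pawn sensing spots a pawn.
; On each sighting it casts player pawn 0 to CharacterController and issues AI MoveTo at that actor, regardless of which pawn was seen.
; It also carries player-style axis bindings for look and movement, separate from the AI chase.
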(event OnSeePawn(PawnSensing)
  (params (Pawn :type Pawn%20Object%20Reference))
  (bind _ascharacter_controller (Utilities|Casting|CastToCharacterController (Game|Player|GetPlayerPawn 0)))
  (AI|AIMoveTo self "100.000000, 0, 0" _ascharacter_controller 5.0 false))

(event Input|AxisEvents|InputAxisLookRight&Left
  (params (AxisValue :type Float%20%28single-precision%29))
  ;[0.05448 0 1] Character Movement
  ;;[1 1 1] Look
  (Pawn|Input|AddControllerYawInput AxisValue))

(event Input|AxisEvents|InputAxisLookUp&Down
  (params (AxisValue :type Float%20%28single-precision%29))
  ;[0.05448 0 1] Character Movement
  ;;[1 1 1] Look
  (Pawn|Input|AddControllerPitchInput AxisValue))

(event Input|AxisEvents|InputAxisMoveForward&Backward
  (params (AxisValue :type Float%20%28single-precision%29))
  ;[0.05448 0 1] Character Movement
  ;;[1 1 1] Movement
  (Pawn|Input|AddMovementInput (Transformation|GetActorForwardVector) AxisValue false))

(event Input|AxisEvents|InputAxisMoveRight&Left
  (params (AxisValue :type Float%20%28single-precision%29))
  ;[0.05448 0 1] Character Movement
  ;;[1 1 1] Movement
  (Pawn|Input|AddMovementInput (Transformation|GetActorRightVector) AxisValue false))

(fn ConstructionScript)