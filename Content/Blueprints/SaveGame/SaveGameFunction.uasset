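; Save game helper functions that store and retrieve the game's settings through a SaveSetings object in the "MySave" slot.
; SaveGameSettings updates the existing save or creates a new one, writes the passed value into its SaveGame field, then saves it to the slot.
; LoadGameSettings returns that field when the slot exists, and returns without setting a value when it does not.
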(fn SaveGameSettings
  (params (SaveGame :type Save%20Game%20Structure%20Structure))
  (bind _returnvalue (SaveGame|DoesSaveGameExist "MySave"))
  (if _returnvalue
    (bind _returnvalue_2 (SaveGame|LoadGamefromSlot "MySave"))
    (bind _assave_game_ (Utilities|Casting|CastToSaveSetings _returnvalue_2))
    (Variables|/Game/Blueprints/SaveGame/SaveSetings.SaveSetings_C|SetSaveGame _assave_game_ SaveGame)
    (SaveGame|SaveGametoSlot _assave_game_ "MySave")
    (else
      (bind _returnvalue_3 (SaveGame|CreateSaveGameObject "/Game/Blueprints/SaveGame/SaveSetings.SaveSetings_C"))
      (Variables|/Game/Blueprints/SaveGame/SaveSetings.SaveSetings_C|SetSaveGame _returnvalue_3 SaveGame)
      (SaveGame|SaveGametoSlot _returnvalue_3 "MySave"))))

(fn LoadGameSettings
  (bind _returnvalue (SaveGame|DoesSaveGameExist "MySave"))
  (if _returnvalue
    (bind _returnvalue_2 (SaveGame|LoadGamefromSlot "MySave"))
    (bind _assave_game_ (Utilities|Casting|CastToSaveSetings _returnvalue_2))
    (return (Variables|/Game/Blueprints/SaveGame/SaveSetings.SaveSetings_C|GetSaveGame _assave_game_))
    (else
      (return ""))))