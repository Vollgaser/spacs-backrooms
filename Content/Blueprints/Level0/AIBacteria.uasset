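; AI enemy for Level 0 that spawns at a random point and emits a periodic bass sound to reveal its location.
; Its first sighting of a pawn triggers a sequence and AIMoveTo chase with audio, then a timed teleport to another spawn.
; Reaching the player disables their movement, turns their view toward the bacteria through a self-calling interpolation loop, fades out and reloads the level.
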(event OnSeePawn(BacteriaSensing)
  (params (Pawn :type Pawn%20Object%20Reference))
  (bind _audio (Variables|Default|GetAudio))
  ;[0 0.9261 1] Random Spawn And Play sound when he sees you
  (Variables|/Script/Engine.CharacterMovementComponent|SetMaxWalkSpeed (Variables|Character|GetCharacterMovement) 605.0)
  (Utilities|FlowControl|DoOnce false
    (:Completed
      (bind _outactor (Sequencer|Player|CreateLevelSequencePlayer "/Game/Blueprints/Level0/Caught_Sequence.Caught_Sequence"))
      (Sequencer|Player|Play (Variables|/Script/LevelSequence.LevelSequenceActor|GetSequencePlayer _outactor) :!class /Script/MovieScene.MovieSceneSequencePlayer)
      (bind _ascharacter_controller (Utilities|Casting|CastToCharacterController Pawn))
      (if (not (Variables|Default|GetCaught?))
        (Variables|Default|SetCan%20see%20enemy? true)
        (if (Variables|Default|GetCan%20see%20enemy?)
          (AI|AIMoveTo self "0, 0, 0" _ascharacter_controller 5.0 false
            (:then
              (Utilities|FlowControl|DoOnce false :!label _label
                (:Completed
                  (Audio|Components|Audio|Play _audio 0.0)
                  (Audio|Components|Audio|FadeOut _audio 5.8 0.0 "Linear" :!class /Script/Engine.AudioComponent)
                  (Utilities|FlowControl|Delay 6.6)
                  (Transformation|SetActorLocation self (.OutItem (Utilities|Array|Random (Variables|Default|GetBacteria%20spawn))) false false)
                  (Variables|Default|SetCan%20see%20enemy? false)
                  (goto _label Reset))))
            (:OnSuccess
              (CallFunction|CatchPlayer))))))))

(event Custom|Catch%20Player
  (bind _returnvalue (Game|GetPlayerController 0))
  ;[0 0.9301 1] Catch
  (Variables|Default|SetCaught? true)
  (Variables|Default|SetShould%20loop true)
  (bind _ascharacter_controller (Utilities|Casting|CastToCharacterController (Game|GetPlayerCharacter 0)))
  (Pawn|Components|CharacterMovement|DisableMovement (Variables|/Script/Engine.Character|GetCharacterMovement _ascharacter_controller))
  (if (Variables|Default|GetShould%20loop)
    (Utilities|FlowControl|Delay 0.001)
    (Transformation|SetActorRotation _ascharacter_controller)
    (Pawn|SetControlRotation _returnvalue (Math|Interpolation|RInterpTo (Pawn|GetControlRotation _returnvalue :!class /Script/Engine.Controller) (Math|Rotator|FindLookatRotation (Transformation|GetActorLocation _ascharacter_controller) (Transformation|GetActorLocation)) (Utilities|Time|GetWorldDeltaSeconds) 5.0))
    (CallFunction|RotatLoop)
    (Utilities|FlowControl|DoOnce false :!label _label
      (:Completed
        (Utilities|FlowControl|Sequence
          (:then_0
            (Utilities|FlowControl|Delay 1.0)
            (CameraFades|StartCameraFade :self (Game|GetPlayerCameraManager 0) :ToAlpha 1.0 :Duration 2.0 :bShouldFadeAudio true :bHoldWhenFinished true)
            (Utilities|FlowControl|Delay 2.1)
            (Game|OpenLevel(byObjectReference) "/Game/Levels/Level_0.Level_0")
            (Variables|Default|SetCaught? false))
          (:then_1
            (Utilities|FlowControl|Delay 0.5)
            (Variables|Default|SetShould%20loop false)
            (goto _label Reset)))))))

(event Custom|RotatLoop
  (bind _returnvalue (Game|GetPlayerController 0))
  ;[0 0.9301 1] Catch
  (if (Variables|Default|GetShould%20loop)
    (Utilities|FlowControl|Delay 0.001)
    (Transformation|SetActorRotation (stale Custom|Catch%20Player _ascharacter_controller))
    (Pawn|SetControlRotation _returnvalue (Math|Interpolation|RInterpTo (Pawn|GetControlRotation _returnvalue :!class /Script/Engine.Controller) (Math|Rotator|FindLookatRotation (Transformation|GetActorLocation (stale Custom|Catch%20Player _ascharacter_controller)) (Transformation|GetActorLocation)) (Utilities|Time|GetWorldDeltaSeconds) 5.0))
    (CallFunction|RotatLoop)
    (Utilities|FlowControl|DoOnce false :!label _label
      (:Completed
        (Utilities|FlowControl|Sequence
          (:then_0
            (Utilities|FlowControl|Delay 1.0)
            (CameraFades|StartCameraFade :self (Game|GetPlayerCameraManager 0) :ToAlpha 1.0 :Duration 2.0 :bShouldFadeAudio true :bHoldWhenFinished true)
            (Utilities|FlowControl|Delay 2.1)
            (Game|OpenLevel(byObjectReference) "/Game/Levels/Level_0.Level_0")
            (Variables|Default|SetCaught? false))
          (:then_1
            (Utilities|FlowControl|Delay 0.5)
            (Variables|Default|SetShould%20loop false)
            (goto _label Reset)))))))

(event EventBeginPlay
  ;[0 0.9301 1] Audio reference
  (bind _returnvalue (AddComponent|AddAudioComponent false))
  (Audio|Components|Audio|Stop _returnvalue)
  (Variables|Default|SetAudio _returnvalue)
  (Transformation|SetActorLocation self (.OutItem (Utilities|Array|Random (Variables|Default|GetBacteria%20spawn))) false false))

(event EventTick
  (params (DeltaSeconds :type Float%20%28single-precision%29))
  ;[0 0.9301 1] Play sound to spot bacteria
  (if (not (Variables|Default|GetCan%20see%20enemy?))
    (Utilities|FlowControl|Delay 4.0)
    (Audio|PlaySoundatLocation "/Game/Assets/Sounds/Level0/Sounds/hard-hitter-808-sub-bass.hard-hitter-808-sub-bass" (Transformation|GetActorLocation) "0, 0, 0" 1.0 1.0 0.0 0 0 0 0)))

(event Input|AxisEvents|InputAxisLookRight&Left
  (params (AxisValue :type Float%20%28single-precision%29))
  ;[0.05448 0 1] Character Movement
  ;;[1 1 1] Look
  (Pawn|Input|AddControllerYawInput AxisValue))

(event Input|AxisEvents|InputAxisLookUp&Down
  (params (AxisValue :type Float%20%28single-precision%29))
  ;[0.05448 0 1] Character Movement
  ;;[1 1 1] Look
  (Pawn|Input|AddControllerPitchInput AxisValue))

(event Input|AxisEvents|InputAxisMoveForward&Backward
  (params (AxisValue :type Float%20%28single-precision%29))
  ;[0.05448 0 1] Character Movement
  ;;[1 1 1] Movement
  (Pawn|Input|AddMovementInput (Transformation|GetActorForwardVector) AxisValue false))

(event Input|AxisEvents|InputAxisMoveRight&Left
  (params (AxisValue :type Float%20%28single-precision%29))
  ;[0.05448 0 1] Character Movement
  ;;[1 1 1] Movement
  (Pawn|Input|AddMovementInput (Transformation|GetActorRightVector) AxisValue false))

(fn ConstructionScript)